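; BP_Enemy_Levitating is a side-scroller enemy that moves along a configurable path and kills the player character on contact.
; The construction script feeds an InterpToMovement component two relative control points from Loc2 and Loc1, plus a travel Duration.
; On overlap it destroys the SideScrollerCharacter, adds an audio component, then reloads the current level by name after a short delay.
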(event EventBeginPlay)

(event Collision|EventActorBeginOverlap
  (params (OtherActor :type Actor%20Object%20Reference))
  (bind _asside_scroller_character (Utilities|Casting|CastToSideScrollerCharacter OtherActor))
  (Actor|DestroyActor _asside_scroller_character)
  (AddComponent|AddAudioComponent false)
  (Utilities|FlowControl|Delay 4.0)
  (bind _returnvalue (Game|GetCurrentLevelName true))
  (Game|OpenLevel(byName) (Utilities|String|StringToName _returnvalue)))

(event EventTick
  (params (DeltaSeconds :type Float%20%28single-precision%29)))

(fn ConstructionScript
  (bind _interptomovement (Variables|Default|GetInterpToMovement))
  (Variables|/Script/Engine.InterpToMovementComponent|SetControlPoints _interptomovement (Utilities|Array|MakeArray (Utilities|Struct|MakeInterpControlPoint (Variables|Default|GetLoc2) true) (Utilities|Struct|MakeInterpControlPoint (Variables|Default|GetLoc1) true)))
  (Variables|/Script/Engine.InterpToMovementComponent|SetDuration _interptomovement (Variables|Default|Getduration)))